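; BP_Turret is an enemy turret that shoots at the player character and can be destroyed.
; When PawnSensing sees a BP_FirstPersonCharacter, it snaps its rotation toward them and, after a short Delay that also throttles fire, spawns a BP_Bullet at the BulletSpawner transform.
; Incoming damage is forwarded to a health component when CanBeDamaged is set, and that component's OnDeath event destroys the actor.
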(event OnSeePawn(PawnSensing)
  (params (Pawn :type Pawn%20Object%20Reference))
  (bind _asbp_first_person_character (Utilities|Casting|CastToBP_FirstPersonCharacter Pawn))
  (Utilities|FlowControl|Sequence
    (:then_0
      (Transformation|SetActorRotation (Math|Rotator|FindLookatRotation (Transformation|GetActorLocation) (Transformation|GetActorLocation _asbp_first_person_character))))
    (:then_1
      (Utilities|FlowControl|Delay 0.5)
      (Game|SpawnActorfromClass "/Game/Enemy/Turret/BP_Bullet.BP_Bullet_C" (Transformation|GetWorldTransform (Variables|Default|GetBulletSpawner)) "Undefined" 0 0))))

(event OnDeath(BP_AC_HealthComponent)
  (Actor|DestroyActor))

(event EventBeginPlay)

(event Collision|EventActorBeginOverlap
  (params (OtherActor :type Actor%20Object%20Reference)))

(event EventTick
  (params (DeltaSeconds :type Float%20%28single-precision%29)))

(event Game|Damage|EventAnyDamage
  (params (Damage :type Float%20%28single-precision%29) (DamageType :type Damage%20Type%20Object%20Reference) (InstigatedBy :type Controller%20Object%20Reference) (DamageCauser :type Actor%20Object%20Reference))
  (if (Variables|Default|GetCanBeDamaged)
    (Default|TakeDamage (Variables|Default|GetBP_AC_HealthComponent) Damage)))

(fn ConstructionScript)