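; AI controller for BP_AI_Enemy that runs its behavior tree and applies timed slow and stun effects.
; BeginPlay seeds two hardcoded blackboard locations, and AI perception writes every updated actor as the target.
; Slows scale walk speed and stuns set a blackboard flag, each reverted by a timer event.
; Tick calls RunBehaviorTree again whenever Blackholed is false, with a trailing Delay that gates nothing.
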(event OnTargetPerceptionUpdated(AIPerception)
  (params (Actor :type Actor%20Object%20Reference) (Stimulus :type AI%20Stimulus%20Structure))
  (AI|Components|Blackboard|SetValueasObject (AI|GetBlackboard 0) (Utilities|Name|MakeLiteralName "Target actor") Actor))

(event Custom|EndSlowly
  (bind _asbp_ai_enemy (Utilities|Casting|CastToBP_AI_Enemy (Pawn|GetControlledPawn)))
  (Utilities|Time|PauseTimerbyHandle (stale Custom|StartSlowly _returnvalue))
  (Variables|/Script/Engine.CharacterMovementComponent|SetMaxWalkSpeed (Variables|/Script/Engine.Character|GetCharacterMovement _asbp_ai_enemy) (Variables|/Game/Enemy/BP_AI_Enemy.BP_AI_Enemy_C|GetMaxSpeed _asbp_ai_enemy)))

(event Custom|StartSlowly
  (params (Time :type Float%20%28double-precision%29) (SpeedKoef :type Float%20%28double-precision%29))
  (bind _asbp_ai_enemy (Utilities|Casting|CastToBP_AI_Enemy (Pawn|GetControlledPawn)))
  (Variables|/Script/Engine.CharacterMovementComponent|SetMaxWalkSpeed (Variables|/Script/Engine.Character|GetCharacterMovement _asbp_ai_enemy) (* (Variables|/Game/Enemy/BP_AI_Enemy.BP_AI_Enemy_C|GetMaxSpeed _asbp_ai_enemy) SpeedKoef))
  (bind _returnvalue (Utilities|Time|SetTimerbyEvent (delegate Custom|EndSlowly) Time))
  (Variables|Default|SetTimer _returnvalue))

(event Custom|Stun
  (Utilities|Time|PauseTimerbyHandle (stale Custom|Starting%20stun _returnvalue))
  (AI|Components|Blackboard|SetValueasBool (AI|GetBlackboard 0) (Utilities|Name|MakeLiteralName "Stunned") false))

(event Custom|Starting%20stun
  (params (Time%20Stun :type Float%20%28double-precision%29))
  (AI|Components|Blackboard|SetValueasBool (AI|GetBlackboard 0) (Utilities|Name|MakeLiteralName "Stunned") true)
  (bind _returnvalue (Utilities|Time|SetTimerbyEvent (delegate Custom|Stun) Time%20Stun))
  (Variables|Default|SetTimer _returnvalue))

(event EventBeginPlay
  (AI|RunBehaviorTree "/Game/Enemy/BT_AI_Enemy.BT_AI_Enemy")
  (AI|Components|Blackboard|SetValueasVector (AI|GetBlackboard 0) (Utilities|Name|MakeLiteralName "Location1") "1600.000000,740.000000,40.000000")
  (AI|Components|Blackboard|SetValueasVector (AI|GetBlackboard 0) (Utilities|Name|MakeLiteralName "Location2") "1600.000000,240.000000,40.000000"))

(event EventTick
  (params (DeltaSeconds :type Float%20%28single-precision%29))
  (if (not (Variables|Default|GetBlackholed))
    (AI|RunBehaviorTree "/Game/Enemy/BT_AI_Enemy.BT_AI_Enemy")
    (Variables|Default|SetBlackholed false)
    (Utilities|FlowControl|Delay 1.0)))

(fn ConstructionScript)