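; BP_Kamikaze is an enemy that explodes when its sphere overlaps the first-person player, launching them away, damaging their health component and destroying itself.
; Tick writes the player's location to the blackboard key "location1", or its own location while the "Stunned" key is set.
; Tick also toggles the stun effect and turns a health readout toward the player.
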(event OnComponentBeginOverlap(Sphere1)
  (params (OverlappedComponent :type Primitive%20Component%20Object%20Reference) (OtherActor :type Actor%20Object%20Reference) (OtherComp :type Primitive%20Component%20Object%20Reference) (OtherBodyIndex :type Integer) (bFromSweep :type Boolean) (SweepResult :type Hit%20Result%20Structure%20%28by%20ref%29))
  (bind _asbp_first_person_character (Utilities|Casting|CastToBP_FirstPersonCharacter OtherActor))
  (Rendering|SetVisibility (Variables|Default|GetCapsuleComponent) false true)
  (Niagara|SpawnSystematLocation "/Game/Enemy/VFX/NS_Enemy_Explotion.NS_Enemy_Explotion" (Transformation|GetActorLocation))
  (Physics|AddImpulse (Variables|/Script/Engine.Character|GetCharacterMovement _asbp_first_person_character) (* (Math|Vector|Normalize (- (Transformation|GetActorLocation OtherActor) (Transformation|GetActorLocation))) (Variables|Default|Getimpulse)) true)
  (Default|TakeDamage (Variables|/Game/FirstPerson/Blueprints/BP_FirstPersonCharacter.BP_FirstPersonCharacter_C|GetBP_AC_HealthComponent _asbp_first_person_character) (Variables|Default|GetDamage))
  (Actor|DestroyActor))

(event EventBeginPlay
  (|CallParentFunction) ; This node is disabled and will not be called.\nDrag off pins to build functionality.
)

(event Collision|EventActorBeginOverlap
  (params (OtherActor :type Actor%20Object%20Reference))
  (|CallParentFunction OtherActor) ; This node is disabled and will not be called.\nDrag off pins to build functionality.
)

(event EventTick
  (params (DeltaSeconds :type Float%20%28single-precision%29))
  (bind _returnvalue (Utilities|Name|MakeLiteralName "location1"))
  (bind _returnvalue_2 (AI|GetBlackboard 0))
  (bind _ns_stun (Variables|Default|GetNS_Stun))
  (bind _textrender (Variables|Default|GetTextRender))
  (Transformation|SetWorldRotation _textrender (Math|Rotator|FindLookatRotation (Transformation|GetActorLocation) (Transformation|GetActorLocation (Game|GetPlayerCharacter 0))) false false)
  (Rendering|Components|TextRender|SetText _textrender (Utilities|Text|ToText(Float) (Variables|/Game/FirstPerson/Blueprints/ActorComponents/BP_AC_HealthComponent.BP_AC_HealthComponent_C|GetHealth (Variables|Default|GetBP_AC_HealthComponent)) "HalfToEven"))
  (if (ScalableFloat|GetValueasBool (AI|GetBlackboard 0) (Utilities|Name|MakeLiteralName "Stunned"))
    (Rendering|SetVisibility _ns_stun true false)
    (AI|Components|Blackboard|SetValueasVector _returnvalue_2 _returnvalue (Transformation|GetActorLocation))
    (else
      (Rendering|SetVisibility _ns_stun false false)
      (AI|Components|Blackboard|SetValueasVector _returnvalue_2 _returnvalue (Transformation|GetActorLocation (Game|GetPlayerCharacter 0))))))

(fn ConstructionScript
  (|CallParentFunction))