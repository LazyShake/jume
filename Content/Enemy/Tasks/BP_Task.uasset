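; Behavior tree task that picks a position for an enemy at a set radius from the first player character.
; When the pawn is farther than Radius, it writes the point on that radius along the player-to-pawn direction into a blackboard vector key.
; Within the radius it leaves the key untouched, and the task finishes successfully either way.
; A random navigable point lookup remains in the graph but is unused.
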(event EventReceiveExecuteAI
  (params (OwnerController :type AI%20Controller%20Object%20Reference) (ControlledPawn :type Pawn%20Object%20Reference))
  (bind _returnvalue (Transformation|GetActorLocation ControlledPawn))
  (bind _returnvalue_2 (Game|GetPlayerCharacter 0))
  (bind _radius (Variables|Default|GetRadius))
  (bind _returnvalue_3 (Transformation|GetActorLocation _returnvalue_2))
  (bind _returnvalue_4 (- _returnvalue _returnvalue_3))
  (if (<= (Math|Vector|VectorLength _returnvalue_4) _radius)
    _
    (else
      (AI|BehaviorTree|SetBlackboardValueasVector (Variables|Default|GetKey) (+ _returnvalue_3 (* (Math|Vector|Normalize _returnvalue_4) _radius)))))
  (AI|BehaviorTree|FinishExecute true))