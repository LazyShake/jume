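; AI enemy character that keeps a set radius from the player, can be stunned and shoots bullets.
; A health component takes damage and destroys the actor on death, while floating text shows health and faces the player.
; Tick writes the blackboard move point near the player, or its own location when stunned, toggling stun VFX.
; Shot rotates toward a velocity-based lead point on the passed target, then spawns a bullet.
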(event OnDeath(BP_AC_HealthComponent)
  (Actor|DestroyActor))

(event EventBeginPlay
  (Variables|/Script/Engine.CharacterMovementComponent|SetMaxWalkSpeed (Variables|Character|GetCharacterMovement) (Variables|Default|GetMaxSpeed))
  (Transformation|SetWorldRotation (Variables|Default|GetP_SmokeVortex1) (Math|Rotator|MakeRotator 0.0 0.0 (Math|Random|RandomFloat)) false false))

(event Collision|EventActorBeginOverlap
  (params (OtherActor :type Actor%20Object%20Reference)))

(event Game|Damage|EventAnyDamage
  (params (Damage :type Float%20%28single-precision%29) (DamageType :type Damage%20Type%20Object%20Reference) (InstigatedBy :type Controller%20Object%20Reference) (DamageCauser :type Actor%20Object%20Reference))
  (if (Variables|Default|GetCanBeDamaged)
    (Default|TakeDamage (Variables|Default|GetBP_AC_HealthComponent) Damage)
    (Development|PrintString "Hello")))

(event EventTick
  (params (DeltaSeconds :type Float%20%28single-precision%29))
  (bind _returnvalue (Utilities|Name|MakeLiteralName "location1"))
  (bind _returnvalue_2 (AI|GetBlackboard 0))
  (bind _returnvalue_3 (Game|GetPlayerCharacter 0))
  (bind _textrender (Variables|Default|GetTextRender))
  (bind _ns_stun (Variables|Default|GetNS_Stun))
  (bind _returnvalue_4 (Transformation|GetActorLocation _returnvalue_3))
  (Transformation|SetWorldRotation _textrender (Math|Rotator|FindLookatRotation (Transformation|GetActorLocation) (Transformation|GetActorLocation (Game|GetPlayerCharacter 0))) false false)
  (Rendering|Components|TextRender|SetText _textrender (Utilities|Text|ToText(Float) (Variables|/Game/FirstPerson/Blueprints/ActorComponents/BP_AC_HealthComponent.BP_AC_HealthComponent_C|GetHealth (Variables|Default|GetBP_AC_HealthComponent)) "HalfToEven"))
  (if (ScalableFloat|GetValueasBool (AI|GetBlackboard 0) (Utilities|Name|MakeLiteralName "Stunned"))
    (Rendering|SetVisibility _ns_stun true false)
    (AI|Components|Blackboard|SetValueasVector _returnvalue_2 _returnvalue (Transformation|GetActorLocation))
    (else
      (Rendering|SetVisibility _ns_stun false false)
      (AI|Components|Blackboard|SetValueasVector _returnvalue_2 _returnvalue (+ _returnvalue_4 (* (Math|Vector|Normalize (- (Transformation|GetActorLocation) _returnvalue_4)) (Variables|Default|GetRadius)))))))

(fn ConstructionScript)

(fn Shot
  (params (NewParam :type BP%20First%20Person%20Character%20Object%20Reference))
  (for _index (range 0 1)
    (Transformation|SetActorRotation (Math|Rotator|FindLookatRotation (Transformation|GetWorldLocation (Variables|Default|GetBulletSpawner)) (+ (Transformation|GetActorLocation NewParam) (/ (* (Transformation|GetActorForwardVector NewParam) (Transformation|GetVelocity NewParam)) "3.000000,3.000000,3.000000")))))
  (Game|SpawnActorfromClass "/Game/Enemy/Turret/BP_Bullet.BP_Bullet_C" (Transformation|GetWorldTransform (Variables|Default|GetBulletSpawner)) "Undefined" 0 0)
  (Audio|PlaySoundatLocation "/Game/Enemy/Sound/weapons-rifle-single-shots-06_Cue.weapons-rifle-single-shots-06_Cue" "0, 0, 0" "0, 0, 0" 1.0 1.0 0.0 0 0 0 0))

(fn Shot1)