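; Flying enemy that locks onto the first player character it sees, pursues it, and shoots while strafing within attack range.
; Tick drives movement and smoothed facing, while a randomly re-armed timer flips strafe direction.
; Shott snaps aim using a rough velocity-based lead before spawning a bullet, throttled by a short delay.
; A blackboard Stunned flag halts behavior and shows an effect; death awards player points and destroys the actor.
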(event OnSeePawn(PawnSensing)
  (params (Pawn :type Pawn%20Object%20Reference))
  (Variables|Default|GetTarget
    (:then)
    (:else
      (bind _asbp_first_person_character (Utilities|Casting|CastToBP_FirstPersonCharacter Pawn))
      (Variables|Default|SetTarget _asbp_first_person_character))))

(event OnDeath(BP_AC_HealthComponent)
  (bind _asbp_first_person_character (Utilities|Casting|CastToBP_FirstPersonCharacter (Game|GetPlayerCharacter 0)))
  (Default|PointsUp _asbp_first_person_character (Variables|Default|GetPoint_0))
  (Actor|DestroyActor))

(event Custom|Fire
  (CallFunction|Shott))

(event Custom|ChangeStrafeDirection
  (bind _isa (Utilities|FlowControl|FlipFlop)
    (:A
      _)
    (:B
      _))
  (Variables|Default|SetStrafeRight _isa)
  (Utilities|Time|SetTimerbyEvent (delegate Custom|ChangeStrafeDirection) (Math|Random|RandomFloatinRange 2.0 4.0)))

(event EventBeginPlay
  (CallFunction|ChangeStrafeDirection))

(event Collision|EventActorBeginOverlap
  (params (OtherActor :type Actor%20Object%20Reference))
  (|CallParentFunction OtherActor))

(event EventTick
  (params (DeltaSeconds :type Float%20%28single-precision%29))
  (bind _returnvalue (Transformation|GetActorLocation))
  (bind _ns_stun (Variables|Default|GetNS_Stun))
  (if (ScalableFloat|GetValueasBool (AI|GetBlackboard 0) (Utilities|Name|MakeLiteralName "Stunned"))
    (Rendering|SetVisibility _ns_stun true false)
    (else
      (Rendering|SetVisibility _ns_stun false false)
      (bind _target (Variables|Default|GetTarget)
        (:then
          (if (> (Transformation|GetDistanceTo _target) (Variables|Default|GetAttackDistance))
            (Pawn|Input|AddMovementInput (Math|Rotator|GetRotationXVector (Math|Rotator|FindLookatRotation _returnvalue (Transformation|GetActorLocation _target))) 1.0 false)
            (Transformation|SetActorRotation (Math|Rotator|Lerp(Rotator) (Transformation|GetActorRotation) (Math|Rotator|FindLookatRotation _returnvalue (Transformation|GetActorLocation _target)) 0.1 true))
            (else
              (Pawn|Input|AddMovementInput (Math|Vector|GetRightVector (Math|Rotator|FindLookatRotation _returnvalue (Transformation|GetActorLocation _target))) (Math|Float|SelectFloat 0.5 -0.5 (Variables|Default|GetStrafeRight)) false)
              (Transformation|SetActorRotation (Math|Rotator|Lerp(Rotator) (Transformation|GetActorRotation) (Math|Rotator|FindLookatRotation _returnvalue (Transformation|GetActorLocation _target)) 0.1 true))
              (if (Variables|Default|GetCan%20Attack)
                (Variables|Default|SetCan%20Attack false)
                (CallFunction|Fire)
                (Utilities|FlowControl|Delay 0.3)
                (Variables|Default|SetCan%20Attack true)))))
        (:else)))))

(fn ConstructionScript
  (|CallParentFunction))

(fn Shott
  (if (not (ScalableFloat|GetValueasBool (AI|GetBlackboard 0) (Utilities|Name|MakeLiteralName "Stunned")))
    (for _index (range 0 1)
      (Transformation|SetActorRotation (Math|Rotator|FindLookatRotation (Transformation|GetWorldLocation (Variables|Default|GetBulletSpawner)) (+ (Transformation|GetActorLocation (Variables|Default|GetTarget)) (/ (* (Transformation|GetActorForwardVector (Variables|Default|GetTarget)) (Transformation|GetVelocity (Variables|Default|GetTarget))) "3.000000,3.000000,3.000000")))))
    (Game|SpawnActorfromClass (Variables|Default|GetBulletClass) (Transformation|GetWorldTransform (Variables|Default|GetBulletSpawner)) "Undefined" 0 0)
    (Audio|PlaySoundatLocation "/Game/Enemy/Sound/FlyingEnemyShot.FlyingEnemyShot" "0, 0, 0" "0, 0, 0" 1.0 1.0 0.0 0 0 0 0)))