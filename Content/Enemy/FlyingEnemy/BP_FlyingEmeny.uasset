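; Flying enemy that drifts between four arrow-marked points while continuously firing BP_Bullet at the player.
; Every few seconds it picks a random arrow and yaw spin, which Tick applies to the mesh.
; A self-rescheduling timer eases the mesh toward that point by lerping from its current location.
; A looping delay drives aimed shots, and damage feeds a health component whose death event destroys the actor.
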(event OnDeath(BP_AC_HealthComponent)
  (Actor|DestroyActor))

(event Custom|Moving
  (bind _staticmesh (Variables|Default|GetStaticMesh))
  (Variables|Default|SetAlpha 0.0)
  (Utilities|Time|SetTimerbyEvent (delegate Custom|Moving) 0.02)
  (Variables|Default|SetAlpha (+ (Variables|Default|GetAlpha) 0.025))
  (Transformation|SetWorldLocation _staticmesh (Math|Vector|Lerp(Vector) (Transformation|GetWorldLocation _staticmesh) (Variables|Default|GetLocationToMove) (Variables|Default|GetAlpha)) false false))

(event Custom|Find%20New%20Location
  (bind _arrow (Variables|Default|GetArrow))
  (bind _arrow2 (Variables|Default|GetArrow2))
  (bind _arrow3 (Variables|Default|GetArrow3))
  (bind _arrow1 (Variables|Default|GetArrow1))
  (bind _array (Utilities|Array|MakeArray _arrow _arrow2 _arrow3 _arrow1))
  (Variables|Default|SetDelta%20Rotation%20Z%20%28Yaw%29 (Math|Random|RandomFloatinRange -2.0 2.0))
  (Variables|Default|SetLocationToMove (Transformation|GetWorldLocation (Utilities|Array|Get(acopy) _array (Math|Random|RandomIntegerinRange 0 (Utilities|Array|LastIndex _array)))))
  (CallFunction|Moving)
  (Utilities|FlowControl|Delay (Math|Random|RandomFloatinRange 2.0 4.0))
  (CallFunction|FindNewLocation))

(event EventBeginPlay
  (CallFunction|FindNewLocation)
  (CallFunction|Shot :!label _label)
  (Utilities|FlowControl|Delay 0.2)
  (goto _label))

(event Collision|EventActorBeginOverlap
  (params (OtherActor :type Actor%20Object%20Reference)))

(event EventTick
  (params (DeltaSeconds :type Float%20%28single-precision%29))
  (Transformation|AddLocalRotation (Variables|Default|GetStaticMesh) (Math|Rotator|MakeRotator 0.0 0.0 (Variables|Default|GetDelta%20Rotation%20Z%20%28Yaw%29)) false false))

(event Game|Damage|EventAnyDamage
  (params (Damage :type Float%20%28single-precision%29) (DamageType :type Damage%20Type%20Object%20Reference) (InstigatedBy :type Controller%20Object%20Reference) (DamageCauser :type Actor%20Object%20Reference))
  (if (Variables|Actor|GetbCanBeDamaged)
    (Default|TakeDamage (Variables|Default|GetBP_AC_HealthComponent) Damage)))

(fn ConstructionScript)

(fn Shot
  (Transformation|SetWorldRotation (Variables|Default|GetBulletSpawner) (Math|Rotator|FindLookatRotation (Transformation|GetWorldLocation (Variables|Default|GetBulletSpawner)) (Transformation|GetWorldLocation (Variables|/Script/Engine.Actor|GetRootComponent (Game|Player|GetPlayerPawn 0)))) false false)
  (Game|SpawnActorfromClass "/Game/Enemy/Turret/BP_Bullet.BP_Bullet_C" (Transformation|GetWorldTransform (Variables|Default|GetBulletSpawner)) "Undefined" 0 0))