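; Behavior tree task that steers a flying enemy toward the player.
; On execute, it casts the controlled pawn to Character and sets its movement component's velocity along the unit direction to a point above player 0, offset by Elevation and scaled by the Velocity variable.
; It finishes successfully right away, so each run is a one-shot velocity update, and a failed cast stops it before it finishes.
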(event EventReceiveExecuteAI
  (params (OwnerController :type AI%20Controller%20Object%20Reference) (ControlledPawn :type Pawn%20Object%20Reference))
  (bind _output_get (Variables|Default|SetControlled%20Pawn ControlledPawn))
  (bind _ascharacter (Utilities|Casting|CastToCharacter _output_get))
  (Variables|Default|SetCharacter%20MovementRef (Variables|/Script/Engine.Character|GetCharacterMovement _ascharacter))
  (Variables|/Script/Engine.MovementComponent|SetVelocity (Variables|Default|GetCharacter%20MovementRef) (* (Math|Vector|GetUnitDirection(Vector) (Transformation|GetActorLocation (Variables|Default|GetControlled%20Pawn)) (+ (Transformation|GetActorLocation (Game|GetPlayerCharacter 0)) (Math|Vector|MakeVector 0.0 0.0 (Variables|Default|GetElevation)))) (Variables|Default|GetVelocity)))
  (AI|BehaviorTree|FinishExecute true))